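; Interactive trigger box that applies an effect to an overlapping BP_TopDownCharacter, chosen by its InteractiveBoxType, and tints its own mesh with Color at BeginPlay.
; Effects swap the character's materials for a dynamic one, set its BigHead flag, or spawn an anchored HandCube.
; The Reset type clears all three, restoring materials from OriginalMaterials, which only the Change Color effect fills on its own box instance.
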(event `self.ReceiveBeginPlay`
  (bind _returnvalue (`PrimitiveComponent.CreateDynamicMaterialInstance` (`self.StaticMesh`) 0 "/Engine/BasicShapes/BasicShapeMaterial.BasicShapeMaterial" "None"))
  (`MaterialInstanceDynamic.SetVectorParameterValue` _returnvalue "Color" (`self.Color`)))

(event `self.ReceiveActorBeginOverlap`
  (params (OtherActor :type "Actor Object Reference"))
  (set `self.Other Actor` OtherActor)
  (switch `/Game/Blueprints/InteractiveBoxTypes` (`self.interactiveBoxType`)
    (:`NewEnumerator0`
      (`self.DoChangeColorEffect`))
    (:`NewEnumerator1`
      (`self.DoBigHeadEffect`))
    (:`NewEnumerator2`
      (`self.DoAddCubeEffect`))
    (:`NewEnumerator3`
      (`self.DoResetEffect`))))

(fn `DoAddCubeEffect`
  (locals (Character :type "/Game/TopDown/Blueprints/BP_TopDownCharacter Object Reference"))
  (bind _asbp_top_down_character (cast `/Game/TopDown/Blueprints/BP_TopDownCharacter` (`self.Other Actor`)))
  (bind _output_get (set `local.Character` _asbp_top_down_character))
  (if (== (`/Game/TopDown/Blueprints/BP_TopDownCharacter.HandCube` _output_get) null)
    (bind _returnvalue (`|SpawnActorFromClass` "/Game/Blueprints/HandCube.HandCube_C" (`KismetMathLibrary.MakeTransform` (0.0 0.0 0.0)) "AlwaysSpawn" "MultiplyWithRoot" null null))
    (set `/Game/Blueprints/HandCube.AnchorPoint` (`self.Other Actor`) _returnvalue)
    (set `/Game/TopDown/Blueprints/BP_TopDownCharacter.HandCube` _returnvalue (`local.Character`))))

(fn `DoBigHeadEffect`
  (bind _asbp_top_down_character (cast `/Game/TopDown/Blueprints/BP_TopDownCharacter` (`self.Other Actor`)))
  (set `/Game/TopDown/Blueprints/BP_TopDownCharacter.BigHead` true _asbp_top_down_character))

(fn `DoChangeColorEffect`
  (locals (DynamicMaterial :type "MaterialInstanceDynamic Object Reference") (Character :type "/Game/TopDown/Blueprints/BP_TopDownCharacter Object Reference"))
  (bind _dynamicmaterial (`local.DynamicMaterial`))
  (bind _mesh (`Character.Mesh` (`local.Character`)))
  (bind _asbp_top_down_character (cast `/Game/TopDown/Blueprints/BP_TopDownCharacter` (`self.Other Actor`)))
  (set `local.Character` _asbp_top_down_character)
  (bind _returnvalue (`PrimitiveComponent.CreateDynamicMaterialInstance` (`self.StaticMesh`) 0 null "None"))
  (bind _output_get (set `local.DynamicMaterial` _returnvalue))
  (`MaterialInstanceDynamic.SetVectorParameterValue` _output_get "None" (`self.Color`))
  (set `self.OriginalMaterials` (`MeshComponent.GetMaterials` (`Character.Mesh` (`local.Character`))))
  (`PrimitiveComponent.SetMaterial` _mesh 1 _dynamicmaterial)
  (`PrimitiveComponent.SetMaterial` _mesh 0 _dynamicmaterial))

(fn `DoResetEffect`
  (locals (Character :type "/Game/TopDown/Blueprints/BP_TopDownCharacter Object Reference"))
  (bind _asbp_top_down_character (cast `/Game/TopDown/Blueprints/BP_TopDownCharacter` (`self.Other Actor`)))
  (bind _output_get (set `local.Character` _asbp_top_down_character))
  (`self.ResetMaterials` _output_get)
  (`self.Reset Add Cube` _output_get)
  ;[1 1 1] Reset Big Head
  (set `/Game/TopDown/Blueprints/BP_TopDownCharacter.BigHead` false (`local.Character`)))

(fn `Reset Add Cube`
  (params (Character :type "/Game/TopDown/Blueprints/BP_TopDownCharacter Object Reference"))
  (`self.K2_DestroyActor` (`/Game/TopDown/Blueprints/BP_TopDownCharacter.HandCube` Character))
  (set `/Game/TopDown/Blueprints/BP_TopDownCharacter.HandCube` null Character))

(fn `ResetMaterials`
  (params (Character :type "/Game/TopDown/Blueprints/BP_TopDownCharacter Object Reference"))
  (bind _originalmaterials (`self.OriginalMaterials`))
  (bind _mesh (`Character.Mesh` Character))
  (`PrimitiveComponent.SetMaterial` _mesh 0 (`|GetArrayItem` _originalmaterials))
  (`PrimitiveComponent.SetMaterial` _mesh 1 (`|GetArrayItem` _originalmaterials 1)))

(fn `UserConstructionScript`)